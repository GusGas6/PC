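; Dwarf enemy character that wanders between random reachable points until killed and reacts to point damage.
; Each hit updates the health bar widget, flashes an overlay material, spawns blood and launches the character along the shot direction.
; Movement friction is zeroed during knockback, then restored after a retriggerable delay before wandering restarts.
; At zero health it ragdolls with a bone impulse, plays a death sound and removes the bar.
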(event `RandomWalk`
  (`|AIMoveTo` self (`NavigationSystemV1.K2_GetRandomReachablePointInRadius` (`self.K2_GetActorLocation`) 5000.0 null null) null 50.0
    (:`OnSuccess`
      _)
    (:`OnFail`
      _))
  (if (not (`self.Dead`))
    (`self.RandomWalk`)))

(event `self.ReceiveBeginPlay`
  (`self.RandomWalk`))

(event `self.ReceivePointDamage`
  (params (Damage :type "Float (single-precision)") (DamageType :type "DamageType Object Reference") (HitLocation :type "Vector Structure") (HitNormal :type "Vector Structure") (HitComponent :type "PrimitiveComponent Object Reference") (BoneName :type Name) (ShotFromDirection :type "Vector Structure") (InstigatedBy :type "Controller Object Reference") (DamageCauser :type "Actor Object Reference") (HitInfo :type "HitResult Structure (by ref)"))
  (bind (_returnvalue_x _returnvalue_y) (`KismetMathLibrary.BreakVector` (* Damage ShotFromDirection 500.0)))
  (bind _charactermovement (`self.CharacterMovement`))
  (bind _charactermovement_2 (`self.CharacterMovement`))
  (bind _currenthealth (`self.CurrentHealth`))
  (bind _mesh (`self.Mesh`))
  (`|ExecutionSequence`
    (:`then_0`
      (set `self.CurrentHealth` (`KismetMathLibrary.FClamp` (- _currenthealth Damage) 0.0 100.0))
      (`self.UpdateHealth`)
      (if (<= _currenthealth 0.0)
        (`PrimitiveComponent.SetSimulatePhysics` _mesh true)
        (`PrimitiveComponent.SetCollisionEnabled` _mesh "QueryAndPhysics")
        (`PrimitiveComponent.AddImpulse` _mesh (* Damage ShotFromDirection 100.0) BoneName true)
        (set `self.Dead` true)
        (`PrimitiveComponent.SetCollisionEnabled` (`self.CapsuleComponent`) "NoCollision")
        (set `CharacterMovementComponent.GravityScale` 0.0 (`self.CharacterMovement`))
        (set `SkeletalMeshComponent.bPauseAnims` true (`self.Mesh`))
        (`/Engine/EditorBlueprintResources/StandardMacros.DoOnce` false
          (:`Completed`
            (`GameplayStatics.PlaySoundAtLocation` "/Game/SFX/Death1_Cue.Death1_Cue" (`SceneComponent.K2_GetComponentLocation` (`self.Mesh`)) (struct) 1.0 1.0 0.0 null null null null)))))
    (:`then_1`
      (if (not (`self.Dead`))
        (`MeshComponent.SetOverlayMaterial` (`self.Mesh`) "/Game/Materials/EnemyHitOverlayMat.EnemyHitOverlayMat")
        (`KismetSystemLibrary.RetriggerableDelay` 0.1)
        (`MeshComponent.SetOverlayMaterial` (`self.Mesh`) null)))
    (:`then_2`
      (set `CharacterMovementComponent.MaxWalkSpeed` 0.0 _charactermovement_2)
      (set `CharacterMovementComponent.GroundFriction` 0.0 _charactermovement_2)
      (`NavMovementComponent.StopActiveMovement` (`self.CharacterMovement`))
      (set `CharacterMovementComponent.BrakingFrictionFactor` 0.0 _charactermovement_2)
      (`KismetSystemLibrary.DelayUntilNextTick`)
      (`self.LaunchCharacter` (`KismetMathLibrary.MakeVector` _returnvalue_x _returnvalue_y) true true)
      (`KismetSystemLibrary.RetriggerableDelay` 0.5)
      (set `CharacterMovementComponent.MaxWalkSpeed` 100.0 _charactermovement)
      (set `CharacterMovementComponent.BrakingFrictionFactor` 2.0 _charactermovement)
      (`self.RandomWalk`))
    (:`then_3`
      (`GameplayStatics.SpawnEmitterAtLocation` "/Game/VFX/MarketplaceAssets/Realistic_Starter_VFX_Pack_Vol2/Particles/Blood/P_Blood_Splat_Cone_Original.P_Blood_Splat_Cone_Original" HitLocation (`KismetMathLibrary.Conv_VectorToRotator` ShotFromDirection)))))

(event `UpdateHealth`
  (bind _widget (`self.Widget`))
  (bind _currenthealth (`self.CurrentHealth`))
  (`/Engine/EditorBlueprintResources/StandardMacros.IsValid` _widget
    (:`Is Valid`
      (bind _asenemy_hpbar_wbp (cast `/Game/UI/EnemyHPBar_WBP` (`WidgetComponent.GetWidget` _widget)))
      (set `/Game/UI/EnemyHPBar_WBP.HealthOfOwner` (/ _currenthealth 100.0) _asenemy_hpbar_wbp)
      (if (or (<= _currenthealth 0.0) (`self.Dead`))
        (`/Engine/EditorBlueprintResources/StandardMacros.DoOnce` false
          (:`Completed`
            (`ActorComponent.K2_DestroyComponent` (`self.Widget`))))))))

(fn `UserConstructionScript`)